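; Wall flag that reacts to an impulsion (Lunar Wave) by changing the wind motion of its banner material.
; On impulsion, if armed, it creates a dynamic material instance from a test material, and two concurrently started timelines drive wind speed, amplitude and direction.
; After three seconds it swaps to an end material and re-arms.
; A separate debug event computes player-distance values that only disconnected experimental nodes use.
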(event Custom|Event_LW
  (bind _returnvalue (Game|GetPlayerCharacter 0))
  (bind _self self)
  (bind _returnvalue_2 (Transformation|GetActorTransform _returnvalue))
  (bind _returnvalue_3 (Transformation|GetActorTransform _self))
  (bind _location (Math|Transform|BreakTransform _returnvalue_2))
  (bind _returnvalue_4 (- (.z _location) (.z (.location _returnvalue_3))))
  (bind _returnvalue_5 (- (.x _location) (.x (.location _returnvalue_3))))
  (bind _returnvalue_6 (- (.y _location) (.y (.location _returnvalue_3))))
  (bind _returnvalue_7 (Math|Float|Absolute(Float) _returnvalue_4))
  (bind _returnvalue_8 (Math|Float|Absolute(Float) _returnvalue_5))
  (bind _returnvalue_9 (Math|Float|Absolute(Float) _returnvalue_6))
  (Variables|Default|SetDistanceVector (Math|Vector|VectorLength (- (.Location (Math|Transform|BreakTransform (Transformation|GetActorTransform (Game|GetPlayerCharacter 0)))) (.location (Transformation|GetActorTransform self)))))
  (Development|PrintString "evebntt_call")
  (Development|PrintString "3secondeici")
  (Utilities|FlowControl|Delay 3.0)
  (Development|PrintString (Utilities|String|Append "On a une distance global:" "X =" (Utilities|String|ToString(Float) _returnvalue_8) "et Y=" (Utilities|String|ToString(Float) _returnvalue_9) "et Z=" (Utilities|String|ToString(Float) _returnvalue_7)) true true "(R=1.000000,G=0.639458,B=0.000000,A=1.000000)" 1e+01)
  (bind _output_get (Variables|Default|SetVectorEnX (/ 1.0 _returnvalue_8)))
  (bind _output_get_2 (Variables|Default|SetVectorEnY (/ 1.0 _returnvalue_9)))
  (bind _output_get_3 (Variables|Default|SetVectorEnZ (/ 1.0 _returnvalue_7))))

(event Collision|EventActorBeginOverlap
  (params (OtherActor :type Actor%20Object%20Reference)))

(event EventTick
  (params (DeltaSeconds :type Float%20%28single-precision%29)))

(event EventOnImpulsionStarted
  (if (Variables|Default|GetInteractLunarWave)
    (Development|PrintString "test_ici")
    (Variables|Default|SetInteractLunarWave false)
    (Utilities|FlowControl|Sequence
      (:then_0
        ;[1 1 1] marche
        (Rendering|Material|SetMaterial (Variables|Default|GetSM_FlagWallHolder) 0 (Variables|Default|Gettestmat))
        (Development|PrintString "retest")
        (bind _returnvalue (Rendering|Material|CreateDynamicMaterialInstance (Rendering|Material|GetMaterial (Variables|Default|GetSM_FlagWallHolder) 0) "None" "None" :!class /Script/Engine.KismetMaterialLibrary))
        (bind _output_get (Variables|Default|SetMID_Banier _returnvalue))
        (Rendering|Material|SetMaterial (Variables|Default|GetSM_FlagWallHolder) 0 _output_get)
        (Utilities|FlowControl|Sequence
          (:then_0
            (bind _newtrack_0 (Timeline|test_timeline PlayFromStart)
              (:Update
                (Utilities|FlowControl|Sequence
                  (:then_0
                    (Rendering|Material|SetScalarParameterValue (Variables|Default|GetMID_Banier) "Speed_Vent" (* _newtrack_0 (Variables|Default|Get__Speed_Vent)) :!class /Script/Engine.MaterialInstanceDynamic))
                  (:then_1
                    (Rendering|Material|SetScalarParameterValue (Variables|Default|GetMID_Banier) "Amplitude_Vent" (* (Variables|Default|Get__Amplitude_Vent) _newtrack_0) :!class /Script/Engine.MaterialInstanceDynamic))
                  (:then_2
                    (Rendering|Material|SetScalarParameterValue (Variables|Default|GetMID_Banier) "Direction_X_Vent" (Variables|Default|Get__Direction_X_Vent) :!class /Script/Engine.MaterialInstanceDynamic))
                  (:then_3
                    (Rendering|Material|SetScalarParameterValue (Variables|Default|GetMID_Banier) "Direction_Y_Vent" (Variables|Default|Get__Direction_Y_Vent) :!class /Script/Engine.MaterialInstanceDynamic))
                  (:then_4
                    (Rendering|Material|SetScalarParameterValue (Variables|Default|GetMID_Banier) "Direction_Z_Vent" (Variables|Default|Get__Direction_Z_Vent) :!class /Script/Engine.MaterialInstanceDynamic))
                  (:then_6
                    (Variables|Default|SetInteractLunarWave false))))))))
      (:then_1
        (Utilities|FlowControl|Sequence
          (:then_0
            (bind _lerp_transi (Timeline|lerp_end PlayFromStart)
              (:Update
                (Utilities|FlowControl|Sequence
                  (:then_1
                    (Rendering|Material|SetScalarParameterValue (Variables|Default|GetMID_Banier) "Speed_Vent" (Math|Float|Lerp (Variables|Default|Get__Speed_Vent) 0.5 _lerp_transi) :!class /Script/Engine.MaterialInstanceDynamic))
                  (:then_3
                    (Rendering|Material|SetScalarParameterValue (Variables|Default|GetMID_Banier) "Amplitude_Vent" (Math|Float|Lerp (Variables|Default|Get__Amplitude_Vent) 5.0 _lerp_transi) :!class /Script/Engine.MaterialInstanceDynamic))
                  (:then_5
                    (Rendering|Material|SetScalarParameterValue (Variables|Default|GetMID_Banier) "Direction_X_Vent" (Math|Float|Lerp (Variables|Default|Get__Direction_X_Vent) 3.0 _lerp_transi) :!class /Script/Engine.MaterialInstanceDynamic))
                  (:then_7
                    (Rendering|Material|SetScalarParameterValue (Variables|Default|GetMID_Banier) "Direction_Y_Vent" (Math|Float|Lerp (Variables|Default|Get__Direction_Y_Vent) 0.0 _lerp_transi) :!class /Script/Engine.MaterialInstanceDynamic))
                  (:then_9
                    (Rendering|Material|SetScalarParameterValue (Variables|Default|GetMID_Banier) "Direction_Z_Vent" (Math|Float|Lerp (Variables|Default|Get__Direction_Z_Vent) 0.0 _lerp_transi) :!class /Script/Engine.MaterialInstanceDynamic))))))
          (:then_1
            (Utilities|FlowControl|Delay 3.0)
            (Rendering|Material|SetMaterial (Variables|Default|GetSM_FlagWallHolder) 0 (Variables|Default|GetEND_MAT))
            (Variables|Default|SetInteractLunarWave true)))))))

(fn ConstructionScript
  (if (Variables|Default|GetInteractLunarWave)
    (CallFunction|EventLW)))