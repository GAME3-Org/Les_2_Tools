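; Actor that samples a target actor's surface on BeginPlay with a grid of vertical line traces, standing in for a mesh vertex scan.
; ScanMeshVertices checks SMSimple, derives XY limits from StaticMeshTarget's bounds, then traces complex Visibility downward at every whole unit, with debug drawing.
; Every trace's Location, hit or not, fills the returned VerticesArray.
; ScanDensity is unused, and Z-bound logic is disconnected.
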(event EventBeginPlay
  (CallFunction|ScanMeshVertices))

(event Collision|EventActorBeginOverlap
  (params (OtherActor :type Actor%20Object%20Reference)))

(event EventTick
  (params (DeltaSeconds :type Float%20%28single-precision%29)))

(fn ConstructionScript)

(fn ScanMeshVertices
  (bind _staticmeshtarget (Variables|Default|GetStaticMeshTarget))
  (bind (_origin _boxextent) (Collision|GetActorBounds _staticmeshtarget false false))
  (bind (_x _y _z) (Math|Vector|BreakVector _origin))
  (bind (_x_2 _y_2 _z_2) (Math|Vector|BreakVector _boxextent))
  (if (Utilities|IsValid (Variables|Default|GetSM_Simple))
    (Utilities|Array|Clear (Variables|Default|GetVerticesArray))
    (Utilities|FlowControl|Sequence
      (:then_2
        ;[1 1 1] Comment
        (LocalVariables|SetX_Min (- _x _x_2)))
      (:then_3
        (LocalVariables|SetX_Max (+ _x _x_2)))
      (:then_4
        (LocalVariables|SetY_Min (- _y _y_2)))
      (:then_5
        (LocalVariables|SetY_Max (+ _y _y_2)))
      (:then_7
        ;[1 1 1] For Loop X
        (for _index (range (Math|Float|Truncate (LocalVariables|GetX_Min)) (Math|Float|Truncate (LocalVariables|GetX_Max)))
          ;[1 1 1] For Loop Y
          (for _index_2 (range (Math|Float|Truncate (LocalVariables|GetY_Min)) (Math|Float|Truncate (LocalVariables|GetY_Max)))
            (bind _outhit (Collision|LineTraceByChannel (Math|Vector|MakeVector (Math|Conversions|ToFloat(Integer) _index) (Math|Conversions|ToFloat(Integer) _index_2) (+ _z (LocalVariables|GetScanHeight))) (Math|Vector|MakeVector (Math|Conversions|ToFloat(Integer) _index) (Math|Conversions|ToFloat(Integer) _index_2) (- _z (* (LocalVariables|GetScanHeight) 2.0))) "TraceTypeQuery1" true 0 "ForDuration"))
            (Utilities|Array|Add (Variables|Default|GetVerticesArray) (.Location (Collision|BreakHitResult _outhit))))))
      (:then_8
        (return false (Variables|Default|GetVerticesArray))))))